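; BP_Door_Ronde is a door prop that rotates its Porte component in yaw when the Interactwith event fires.
; When locked, it replays a separate timeline from the start without changing the closed state.
; When unlocked, it flips IsClosed and plays or reverses the swing timeline to open or close.
; Both timelines scale their curve output by a negated RotationAngle to set relative rotation.
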(event `/Game/Interactive/BPI_interaction.InteractWith`
  (params (Interactor :type "Actor Object Reference"))
  (if (`self.IsLocked`)
    (bind (_direction _rota) (`Timeline|Timeline` :!via `PlayFromStart`)
      (:`Update`
        (`SceneComponent.K2_SetRelativeRotation` (`self.porte`) (`KismetMathLibrary.MakeRotator` 0.0 0.0 (* _rota (`self.RotationAngle`) -1.0)) false false)))
    (elif (`self.IsClosed`)
      (set `self.IsClosed` false)
      (bind (_direction_2 _rotation) (`Timeline|Timeline_0` :!label _label)
        (:`Update`
          (`SceneComponent.K2_SetRelativeRotation` (`self.porte`) (`KismetMathLibrary.MakeRotator` 0.0 0.0 (* _rotation (`self.RotationAngle`) -1.0)) false false)))
      (else
        (set `self.IsClosed` true)
        (goto _label :!via `Reverse`)))))

(fn `UserConstructionScript`)