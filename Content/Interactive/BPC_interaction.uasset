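; BPC_interaction is an interaction component that finds the interactable actor in front of its owner.
; InteractionTrace runs a short forward sphere trace from the owner's location on a dedicated trace channel, drawing debug shapes for one frame.
; It stores the hit actor in TargetActor if it implements BPI_interaction, otherwise clears it.
; The component's own event graph is empty, so it never calls the trace itself.
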(fn `InteractionTrace`
  (bind _returnvalue (`self.GetOwner`))
  (bind _returnvalue_2 (`Actor.K2_GetActorLocation` _returnvalue))
  (bind (_outhit _returnvalue_3) (`KismetSystemLibrary.SphereTraceSingle` :`Start` _returnvalue_2 :`End` (+ _returnvalue_2 (* (`Actor.GetActorForwardVector` _returnvalue) 100.0)) :`Radius` 50.0 :`TraceChannel` "TraceTypeQuery3" :`DrawDebugType` "ForOneFrame"))
  (if _returnvalue_3
    (bind (_bblockinghit _binitialoverlap _time _distance _location _impactpoint _normal _impactnormal _physmat _hitactor) (`GameplayStatics.BreakHitResult` _outhit))
    (if (`KismetSystemLibrary.DoesImplementInterface` _hitactor "/Game/Interactive/BPI_interaction.BPI_interaction_C")
      (set `self.TargetActor` _hitactor)
      (else
        (set `self.TargetActor` null)))
    (else
      (set `self.TargetActor` null))))